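; BP_PlayerHUD is an actor that creates the player HUD widget at BeginPlay and acts as its go-between with the game.
; It binds to the widget's change-audio event, rebroadcasts the click through its own ChangeAudioButtonEvent dispatcher, and also applies one point of damage to the player pawn.
; SetLives forwards the lives count to the widget, while a leftover PlayNextAudio and DamagePlayer chain is never run.
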(event `self.ReceiveBeginPlay`
  (bind _returnvalue (`|CreateWidget` "/Game/PlayerHUD.PlayerHUD_C"))
  (bind _output_get (set `self.PlayerHUD Reference` _returnvalue))
  (`UserWidget.AddToViewport` _output_get 0)
  (add `/Game/PlayerHUD.ChangePlayerAudio` (`self.PlayerHUD Reference`) (delegate `Change Audio Button Clicked`)))

(event `Change Audio Button Clicked`
  (`self.Change Audio Button Event`)
  (`self.Damage Player`))

(fn `Damage Player`
  (`GameplayStatics.ApplyDamage` (`GameplayStatics.GetPlayerPawn` 0) 1.0))

(fn `Set Lives`
  (params (Lives :type Integer))
  (`/Game/PlayerHUD.Set Lives` (`self.PlayerHUD Reference`) Lives))

(fn `UserConstructionScript`)